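; BP_MHWCharacter is a character Blueprint that starts play equipped with a Great Sword.
; BeginPlay hands the input mapping asset to the config manager, links the sheathed Great Sword anim layer to the mesh, and equips the sword through MHWEquipmentManagerComponent.
; Linked anim class layers supply the weapon-specific animation.
; Debug aids remain active: BeginPlay opens the Enhanced Input debug display, and Tick prints actor rotation every frame.
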(event `self.ReceiveBeginPlay`
  (`|ExecutionSequence`
    (:`then_0`
      (`KismetSystemLibrary.ExecuteConsoleCommand` "showdebug enhancedinput" null))
    (:`then_1`
      (`ConfigManager.SetInputActionMappingAsset` (subsystem `ConfigManager`) "/Game/_Main/Data/DataAsset/DA_InputMapping.DA_InputMapping")
      (`SkeletalMeshComponent.LinkAnimClassLayers` (`self.Mesh`) "/Game/_Main/Blueprints/AnimationBP/LinkedLayers/GreatSword/ABP_Layer_GreatSword_Sheathed.ABP_Layer_GreatSword_Sheathed_C")
      (`MHWEquipmentManagerComponent.EquipItem` (`self.MHWEquipmentManagerComponent`) "/Game/_Main/Blueprints/Equipment/EquipmentDefination/ED_GreatSword.ED_GreatSword_C"))))

(event `self.ReceiveTick`
  (params (DeltaSeconds :type "Float (single-precision)"))
  (bind _returnvalue (`KismetStringLibrary.Conv_RotatorToString` (`self.K2_GetActorRotation`)))
  (`KismetSystemLibrary.PrintString` _returnvalue true true (struct :`G` 0.66 :`B` 1.0 :`A` 1.0) 0.0 (`KismetStringLibrary.Conv_StringToName` _returnvalue)))

(fn `UserConstructionScript`)