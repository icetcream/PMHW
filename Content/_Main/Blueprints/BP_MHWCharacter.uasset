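; BP_MHWCharacter is a character Blueprint with a sheathed great sword animation layer, linked to its mesh on BeginPlay.
; Left Shift switches max walk speed between scaled base and accelerated velocities.
; For debugging, Tick draws a forward-facing arrow, and keys toggle slow-motion time dilation or play a test montage.
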(event EventBeginPlay
  (Components|SkeletalMesh|AnimationBlueprintLinking|LinkAnimClassLayers (Variables|Character|GetMesh) "/Game/_Main/Blueprints/AnimationBP/LinkedLayers/GreatSword/ABP_Layer_GreatSword_Sheated.ABP_Layer_GreatSword_Sheated_C")
  (Variables|/Script/Engine.CharacterMovementComponent|SetMaxWalkSpeed (Variables|Character|GetCharacterMovement) (* (Variables|Default|GetBaseVel) 2.5)))

(event Collision|EventActorBeginOverlap
  (params (OtherActor :type Actor%20Object%20Reference)))

(event EventTick
  (params (DeltaSeconds :type Float%20%28single-precision%29))
  (bind _returnvalue (Transformation|GetActorLocation))
  (bind _returnvalue_2 (+ _returnvalue "0.000000,0.000000,50.000000"))
  (Rendering|Debug|DrawDebugArrow _returnvalue_2 (+ _returnvalue_2 (* (Transformation|GetActorForwardVector) "50.000000,50.000000,0.000000")) 5.0 "(R=0.995748,G=0.000000,B=1.000000,A=1.000000)" 0.0 5.0))

(event Input|KeyboardEvents|DebugKeyJ
  (params (Key :type Key%20Structure) (ActionValue :type Input%20Action%20Value%20Structure))
  (:Pressed
    (Animation|Montage|PlayMontage (Variables|Character|GetMesh) "/Game/_Main/Character/Animations/BaseLocomotion/AM_129.AM_129")))

(event Input|KeyboardEvents|DebugKey1
  (params (Key :type Key%20Structure) (ActionValue :type Input%20Action%20Value%20Structure))
  (:Pressed
    (Utilities|Time|SetGlobalTimeDilation 0.1)))

(event Input|KeyboardEvents|DebugKey2
  (params (Key :type Key%20Structure) (ActionValue :type Input%20Action%20Value%20Structure))
  (:Pressed
    (Utilities|Time|SetGlobalTimeDilation 1.0)))

(event Input|KeyboardEvents|LeftShift
  (params (Key :type Key%20Structure))
  (:Pressed
    (Variables|/Script/Engine.CharacterMovementComponent|SetMaxWalkSpeed (Variables|Character|GetCharacterMovement) (* (Variables|Default|GetAccVel) 2.5)))
  (:Released
    (Variables|/Script/Engine.CharacterMovementComponent|SetMaxWalkSpeed (Variables|Character|GetCharacterMovement) (* (Variables|Default|GetBaseVel) 2.5))))

(fn ConstructionScript)