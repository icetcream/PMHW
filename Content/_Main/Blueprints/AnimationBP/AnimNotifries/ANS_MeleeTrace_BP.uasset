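; Anim notify state that marks the melee hit-detection window within an attack animation.
; On begin, it gets the owner's melee trace component through MHWCharacterInterface and starts tracing with the notify's base socket and trace sockets.
; On end, it stops that component's trace, so the notify only sets timing and sockets while the component handles the tracing.
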(fn `Received_NotifyBegin`
  (params (MeshComp :type "SkeletalMeshComponent Object Reference") (Animation :type "AnimSequenceBase Object Reference") (TotalDuration :type "Float (single-precision)") (EventReference :type "AnimNotifyEventReference Structure (by ref)"))
  (returns (ReturnValue :type Boolean))
  (bind _asmhwcharacter_interface (cast `MHWCharacterInterface` (`ActorComponent.GetOwner` MeshComp)))
  (bind _returnvalue (`MHWCharacterInterface.GetMeleeTraceComponent` _asmhwcharacter_interface))
  (`MeleeTraceComponent.StartTrace` _returnvalue (`self.In Base Socket`) (`self.In Trace Sockets`))
  (return false))

(fn `Received_NotifyEnd`
  (params (MeshComp :type "SkeletalMeshComponent Object Reference") (Animation :type "AnimSequenceBase Object Reference") (EventReference :type "AnimNotifyEventReference Structure (by ref)"))
  (returns (ReturnValue :type Boolean))
  (bind _asmhwcharacter_interface (cast `MHWCharacterInterface` (`ActorComponent.GetOwner` MeshComp)))
  (bind _returnvalue (`MHWCharacterInterface.GetMeleeTraceComponent` _asmhwcharacter_interface))
  (`MeleeTraceComponent.StopTrace` _returnvalue)
  (return false))